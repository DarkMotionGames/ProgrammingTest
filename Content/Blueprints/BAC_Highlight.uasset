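; BAC_Highlight is a Blueprint component that highlights its owning actor when the mouse cursor hovers over it.
; On BeginPlay it enables mouse-over events on the first player controller, binds to the owner's cursor over events and caches the owner's static mesh component, if valid.
; The hover handlers toggle Render Custom Depth on that mesh, without checking the cached reference again.
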(event Custom|EndHover
  (params (TouchedActor :type Actor%20Object%20Reference))
  (Rendering|SetRenderCustomDepth (Variables|Default|GetStaticMeshRef) false))

(event Custom|MouseHover
  (params (TouchedActor :type Actor%20Object%20Reference))
  (Rendering|SetRenderCustomDepth (Variables|Default|GetStaticMeshRef) true))

(event EventBeginPlay
  (bind _returnvalue (Components|GetOwner))
  (bind _returnvalue_2 (Actor|GetComponentbyClass _returnvalue "/Script/Engine.StaticMeshComponent"))
  (Variables|/Script/Engine.PlayerController|SetbEnableMouseOverEvents (Game|GetPlayerController 0) true)
  (EventDispatchers|BindEventtoOnBeginCursorOver _returnvalue (delegate Custom|MouseHover))
  (EventDispatchers|BindEventtoOnEndCursorOver _returnvalue (delegate Custom|EndHover))
  (Utilities|IsValid _returnvalue_2
    (:Is%20Valid
      (Variables|Default|SetStaticMeshRef _returnvalue_2))))