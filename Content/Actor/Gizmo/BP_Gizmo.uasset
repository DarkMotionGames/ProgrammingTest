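; BP_Gizmo is a translation gizmo actor with X, Y and Z axis handles, toggled by the M key.
; While enabled, a left click traces from the mouse, identifies the hit axis through DetectAxis and stores grab distance and location; release clears the axis.
; Logic to move the SceneComponent along the dragged axis and attach the Mesh exists but is disconnected, and Tick is empty, so nothing moves.
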(event EventBeginPlay
  (Input|EnableInput (Game|GetPlayerController 0)))

(event EventTick
  (params (DeltaSeconds :type Float%20%28single-precision%29)))

(event Input|MouseEvents|LeftMouseButton
  (params (Key :type Key%20Structure :default "None"))
  (bind _returnvalue (Game|GetPlayerController 0))
  (bind (_worldlocation _worlddirection) (Game|Player|ConvertMouseLocationToWorldSpace _returnvalue))
  (:Pressed
    (if (Variables|Default|GetCanMove)
      (bind _outhit (Collision|LineTraceByChannel _worldlocation (+ (* _worlddirection 1e+03) _worldlocation) "TraceTypeQuery1" true 0 "ForDuration" false))
      (Variables|Default|SetDistanceToGrab (.Distance (Collision|BreakHitResult _outhit)))
      (switch Utilities|FlowControl|Switch|SwitchonE_AxisGizmo (.axisvalues (Utilities|Struct|MakeF_GizmoAxis 0 (CallFunction|DetectAxis (.HitComponent (Collision|BreakHitResult _outhit)))))
        (:NewEnumerator0
          (Variables|Default|SetDraggedLocation (Math|Transform|InverseTransformLocation (Math|Conversions|ToTransform(Vector) (Math|Conversions|ToVector(Float) (Class|GameplayStatics|GetWorldOriginLocation))) (.Location (Collision|BreakHitResult _outhit))))
          (Development|PrintString "x"))
        (:NewEnumerator1
          (Variables|Default|SetDraggedLocation (Math|Transform|InverseTransformLocation (Math|Conversions|ToTransform(Vector) (Math|Conversions|ToVector(Float) (Class|GameplayStatics|GetWorldOriginLocation))) (.Location (Collision|BreakHitResult _outhit))))
          (Development|PrintString "y"))
        (:NewEnumerator2
          (Variables|Default|SetDraggedLocation (Math|Transform|InverseTransformLocation (Math|Conversions|ToTransform(Vector) (Math|Conversions|ToVector(Float) (Class|GameplayStatics|GetWorldOriginLocation))) (.Location (Collision|BreakHitResult _outhit))))
          (Development|PrintString "z")))))
  (:Released
    (if (Variables|Default|GetCanMove)
      (Variables|Default|SetAxisDragged 0))))

(event Input|KeyboardEvents|M
  (params (Key :type Key%20Structure :default "None"))
  (bind _returnvalue (Game|GetPlayerController 0))
  (:Pressed
    (Variables|Default|SetCanMove (not (Variables|Default|GetCanMove)))
    (Variables|/Script/Engine.PlayerController|SetbShowMouseCursor _returnvalue (Variables|/Script/Engine.PlayerController|GetbShowMouseCursor _returnvalue))))

(fn ConstructionScript)

(fn DetectAxis
  (params (Primitive%20Comp :type Primitive%20Component%20Object%20Reference))
  (Variables|Default|SetAxisDragged Primitive%20Comp)
  (if (== (Variables|Default|GetAxisDragged) (Variables|Default|GetXAxis))
    (return "NewEnumerator0")
    (elif (== (Variables|Default|GetAxisDragged) (Variables|Default|GetYAxis))
      (return "NewEnumerator1")
      (elif (== (Variables|Default|GetAxisDragged) (Variables|Default|GetZAxis))
        (return "NewEnumerator2")))))