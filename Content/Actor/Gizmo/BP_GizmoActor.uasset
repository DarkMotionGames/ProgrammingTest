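; Translation gizmo actor that lets the player drag it along its world X, Y or Z axis with the mouse.
; While left mouse is held, a looping timer traces from the cursor to pick an axis, storing hit distance and grab offset.
; Tick projects the cursor at that distance, moves SceneComponent along that axis only and disables the other handles' collision until release.
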(event Custom|Mosue%20Pressed
  (bind _returnvalue (Game|GetPlayerController 0))
  (bind (_worldlocation _worlddirection) (Game|Player|ConvertMouseLocationToWorldSpace _returnvalue))
  ;[1 1 1] Select Axis
  (bind _outhit (Collision|LineTraceByChannel _worldlocation (+ (* _worlddirection (Math|Float|MakeLiteralFloat 1e+04)) _worldlocation) "TraceTypeQuery1" true 0 "ForOneFrame" false))
  (if (Math|Boolean|ORBoolean (== (.HitComponent (Collision|BreakHitResult _outhit)) (Variables|Default|GetXAxis)) (== (.HitComponent (Collision|BreakHitResult _outhit)) (Variables|Default|GetYAxis)) (== (.HitComponent (Collision|BreakHitResult _outhit)) (Variables|Default|GetZAxis)))
    (Variables|Default|SetDistance (.Distance (Collision|BreakHitResult _outhit)))
    (switch Utilities|FlowControl|Switch|SwitchonE_AxisGizmo (.axisvalues (Utilities|Struct|MakeF_GizmoAxis 0 (CallFunction|DetectAxis (.HitComponent (Collision|BreakHitResult _outhit)))))
      (:NewEnumerator0
        (Development|PrintString "x")
        (Variables|Default|SetMoveX true)
        (Variables|Default|SetMoveY false)
        (Variables|Default|SetMoveZ false)
        (Variables|Default|SetCanMove true))
      (:NewEnumerator1
        (Development|PrintString "y")
        (Variables|Default|SetMoveX false)
        (Variables|Default|SetMoveY true)
        (Variables|Default|SetMoveZ false)
        (Variables|Default|SetCanMove true))
      (:NewEnumerator2
        (Development|PrintString "z")
        (Variables|Default|SetMoveX false)
        (Variables|Default|SetMoveY false)
        (Variables|Default|SetMoveZ true)
        (Variables|Default|SetCanMove true)))
    (Variables|Default|SetRelativeGrabLocation (Math|Transform|InverseTransformLocation (Math|Conversions|ToTransform(Vector) (Transformation|GetWorldLocation (.HitComponent (Collision|BreakHitResult _outhit)))) (.Location (Collision|BreakHitResult _outhit))))))

(event EventBeginPlay
  ;[1 1 1] Select Axis
  (Input|EnableInput (Game|GetPlayerController 0)))

(event EventTick
  (params (DeltaSeconds :type Float%20%28single-precision%29))
  (Variables|Default|SetCurrent%20Location (Transformation|GetActorLocation))
  (CallFunction|MoveDirection))

(event Input|MouseEvents|LeftMouseButton
  (params (Key :type Key%20Structure :default "None"))
  (:Pressed
    (bind _returnvalue (Utilities|Time|SetTimerbyEvent (delegate Custom|Mosue%20Pressed) 0.1 true true))
    (Variables|Default|SetTimer _returnvalue))
  (:Released
    (Utilities|Time|ClearandInvalidateTimerbyHandle (Variables|Default|GetTimer))
    ;[1 1 1] Select Axis
    (Variables|Default|SetCanMove false)
    (Collision|SetCollisionEnabled (Variables|Default|GetXAxis) "QueryAndPhysics")
    (Collision|SetCollisionEnabled (Variables|Default|GetYAxis) "QueryAndPhysics")
    (Collision|SetCollisionEnabled (Variables|Default|GetZAxis) "QueryAndPhysics")))

(fn ConstructionScript)

(fn DetectAxis
  (params (Primitive%20Comp :type Primitive%20Component%20Object%20Reference))
  (Variables|Default|SetAxisDragged Primitive%20Comp)
  (if (== (Variables|Default|GetAxisDragged) (Variables|Default|GetXAxis))
    (return "NewEnumerator0")
    (elif (== (Variables|Default|GetAxisDragged) (Variables|Default|GetYAxis))
      (return "NewEnumerator1")
      (elif (== (Variables|Default|GetAxisDragged) (Variables|Default|GetZAxis))
        (return "NewEnumerator2")))))

(fn MoveDirection
  (bind _returnvalue (Game|GetPlayerController 0))
  (bind _returnvalue_2 (Game|GetPlayerController 0))
  (bind _returnvalue_3 (Game|GetPlayerController 0))
  (bind _returnvalue_4 (Game|GetPlayerController 0))
  (bind _current_location (Variables|Default|GetCurrent%20Location))
  (bind _current_location_2 (Variables|Default|GetCurrent%20Location))
  (bind _current_location_3 (Variables|Default|GetCurrent%20Location))
  (bind (_worldlocation _worlddirection) (Game|Player|ConvertMouseLocationToWorldSpace _returnvalue))
  (bind (_worldlocation_2 _worlddirection_2) (Game|Player|ConvertMouseLocationToWorldSpace _returnvalue_3))
  (bind (_worldlocation_3 _worlddirection_3) (Game|Player|ConvertMouseLocationToWorldSpace _returnvalue_2))
  (bind (_worldlocation_4 _worlddirection_4) (Game|Player|ConvertMouseLocationToWorldSpace _returnvalue_4))
  (Variables|Default|SetWorldPosition _worldlocation)
  (Variables|Default|SetWorldDirection _worlddirection)
  (if (Variables|Default|GetCanMove)
    (if (Variables|Default|GetMoveX)
      (Transformation|SetWorldLocation (Variables|Default|GetSceneComponent) (Math|Vector|MakeVector (.x (Math|Transform|InverseTransformLocation (Math|Conversions|ToTransform(Vector) (Variables|Default|GetRelativeGrabLocation)) (+ _worldlocation_3 (* _worlddirection_3 (Variables|Default|GetDistance))))) (.y _current_location) (.z _current_location)) false false)
      (Collision|SetCollisionEnabled (Variables|Default|GetYAxis) "NoCollision")
      (Collision|SetCollisionEnabled (Variables|Default|GetZAxis) "NoCollision")
      (elif (Variables|Default|GetMoveY)
        (Transformation|SetWorldLocation (Variables|Default|GetSceneComponent) (Math|Vector|MakeVector (.x _current_location_2) (.y (Math|Transform|InverseTransformLocation (Math|Conversions|ToTransform(Vector) (Variables|Default|GetRelativeGrabLocation)) (+ _worldlocation_4 (* _worlddirection_4 (Variables|Default|GetDistance))))) (.z _current_location_2)) false false)
        (Collision|SetCollisionEnabled (Variables|Default|GetXAxis) "NoCollision")
        (Collision|SetCollisionEnabled (Variables|Default|GetZAxis) "NoCollision")
        (elif (Variables|Default|GetMoveZ)
          (Transformation|SetWorldLocation (Variables|Default|GetSceneComponent) (Math|Vector|MakeVector (.x _current_location_3) (.y _current_location_3) (.z (Math|Transform|InverseTransformLocation (Math|Conversions|ToTransform(Vector) (Variables|Default|GetRelativeGrabLocation)) (+ _worldlocation_2 (* _worlddirection_2 (Variables|Default|GetDistance)))))) false false)
          (Collision|SetCollisionEnabled (Variables|Default|GetYAxis) "NoCollision")
          (Collision|SetCollisionEnabled (Variables|Default|GetXAxis) "NoCollision"))))))